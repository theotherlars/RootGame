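; Launch pad that throws the third-person character diagonally forward and upward when it overlaps the box trigger.
; The overlap plays a timeline that tilts a scene component via a rotator lerp.
; Its first update launches the character along the pad's forward vector plus an upward force, overriding Z velocity.
; A DoOnce limits this to one launch until a delay after the timeline finishes rewinds it and resets the gate.
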(event `self.Box.OnComponentBeginOverlap`
  (params (OverlappedComponent :type "PrimitiveComponent Object Reference") (OtherActor :type "Actor Object Reference") (OtherComp :type "PrimitiveComponent Object Reference") (OtherBodyIndex :type Integer) (bFromSweep :type Boolean) (SweepResult :type "HitResult Structure (by ref)"))
  (bind (_returnvalue_x _returnvalue_y) (`KismetMathLibrary.BreakVector` (`self.GetActorForwardVector`)))
  (bind _asbp_third_person_character (cast `/Game/ThirdPerson/Blueprints/BP_ThirdPersonCharacter` OtherActor))
  (bind (_direction _rotation) (`Timeline|Timeline` :!label _label)
    (:`Update`
      (`SceneComponent.K2_SetRelativeRotation` (`self.Scene`) (`KismetMathLibrary.RLerp` (struct) (struct :`Pitch` -45.0) _rotation) false false)
      (`/Engine/EditorBlueprintResources/StandardMacros.DoOnce` false :!label _label_2
        (:`Completed`
          (`Character.LaunchCharacter` _asbp_third_person_character (`KismetMathLibrary.MakeVector` (* _returnvalue_x (`self.LaunchForce`)) (* _returnvalue_y (`self.LaunchForce`)) (`self.LaunchForce`)) false true))))
    (:`Finished`
      (`KismetSystemLibrary.Delay` 3.0)
      (`|ExecutionSequence`
        (:`then_0`
          (goto _label :!via `SetNewTime`))
        (:`then_1`
          (goto _label_2 :!via `Reset`))))))

(event `self.Box.OnComponentEndOverlap`
  (params (OverlappedComponent :type "PrimitiveComponent Object Reference") (OtherActor :type "Actor Object Reference") (OtherComp :type "PrimitiveComponent Object Reference") (OtherBodyIndex :type Integer)))

(fn `UserConstructionScript`)