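; BP_BoulderSpawner is an actor that slides along a path while continuously spawning BP_Boulder actors at its current position.
; A looping timeline lerps it from its start location toward the EndLocation component's world position, which is re-read each update.
; A separate endless delay loop spawns boulders at random intervals between MinFireRate and MaxFireRate.
; The construction script draws a temporary debug line to EndLocation; the MoveAmount-based EndLoc is computed but unused.
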(event `self.ReceiveBeginPlay`
  (set `self.StartLoc` (`self.K2_GetActorLocation`))
  (set `self.EndLoc` (+ (`self.StartLoc`) (`self.MoveAmount`)))
  (`self.MoveSpawner`)
  (`self.StartSpawnBoulders`))

(event `MoveSpawner`
  (bind (_direction _timeforcanontomove) (`Timeline|Timeline` :!via `PlayFromStart` :!label _label)
    (:`Update`
      (`self.K2_SetActorLocation` (`KismetMathLibrary.VLerp` (`self.StartLoc`) (`SceneComponent.K2_GetComponentLocation` (`self.EndLocation`)) _timeforcanontomove)))
    (:`Finished`
      (goto _label :!via `PlayFromStart`))))

(event `StartSpawnBoulders`
  (`|SpawnActorFromClass` "/Game/MoleGame/Blueprints/BP_Boulder.BP_Boulder_C" (`KismetMathLibrary.MakeTransform` (`self.K2_GetActorLocation`)) "Undefined" "OverrideRootScale" null null :!label _label_2)
  (`KismetSystemLibrary.Delay` (`KismetMathLibrary.RandomFloatInRange` (`self.MinFireRate`) (`self.MaxFireRate`)))
  (goto _label_2))

(fn `UserConstructionScript`
  (`KismetSystemLibrary.DrawDebugLine` (`SceneComponent.K2_GetComponentLocation` (`self.DefaultSceneRoot`)) (`SceneComponent.K2_GetComponentLocation` (`self.EndLocation`)) (struct :`R` 0.901042 :`G` 0.130463 :`B` 0.835304 :`A` 1.0) 5.0 2.0))