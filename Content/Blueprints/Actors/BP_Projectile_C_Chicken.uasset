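; Child projectile Blueprint, named for a chicken, that varies its appearance on each spawn.
; At BeginPlay, after the parent logic, it randomly unhides one of five mesh components: the default StaticMesh or one of four vegetable variants.
; It also gives the Sphere component a random world rotation.
; All other behavior comes from the parent, as the overlap and tick events are disabled stubs.
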(event `self.ReceiveBeginPlay`
  (`parent.ReceiveBeginPlay`)
  (`SceneComponent.SetHiddenInGame` (select `int` (`KismetMathLibrary.RandomIntegerInRange` 0 4) :`0` (`self.StaticMesh`) :`1` (`self.Carrot`) :`2` (`self.Onion`) :`3` (`self.Potato`) :`4` (`self.Tomato`)) false false)
  (`SceneComponent.K2_SetWorldRotation` (`self.Sphere`) (`KismetMathLibrary.RandomRotator` false) false false))

(fn `UserConstructionScript`
  (`parent.UserConstructionScript`))