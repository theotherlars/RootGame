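; BP_PigCanon is a moving cannon actor that continuously fires pig projectiles.
; On BeginPlay it sets a goal at its start location plus a move offset, then starts both movement and firing.
; A timeline lerps the actor between those two points and restarts itself when finished.
; The firing event spawns BP_Projectile_C_Pig at the Arrow component's transform, looping through a Delay set by PigFireRate.
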(event `self.ReceiveBeginPlay`
  (set `self.ActorStartLocation` (`self.K2_GetActorLocation`))
  (set `self.ActorGoalLocation` (+ (`self.ActorStartLocation`) (`self.ActorMoveOffset`)))
  (`self.MoveCanonVertical`)
  (`self.ShootPig`))

(event `MoveCanonVertical`
  (bind (_direction _timeforcanontomove) (`Timeline|Timeline` :!via `PlayFromStart` :!label _label)
    (:`Update`
      (`self.K2_SetActorLocation` (`KismetMathLibrary.VLerp` (`self.ActorStartLocation`) (`self.ActorGoalLocation`) _timeforcanontomove)))
    (:`Finished`
      (goto _label :!via `PlayFromStart`))))

(event `ShootPig`
  (`|SpawnActorFromClass` "/Game/Blueprints/Actors/BP_Projectile_C_Pig.BP_Projectile_C_Pig_C" (`SceneComponent.K2_GetComponentToWorld` (`self.Arrow`)) "Undefined" "OverrideRootScale" null null :!label _label_2)
  (`KismetSystemLibrary.Delay` (`self.PigFireRate`))
  (goto _label_2))

(fn `UserConstructionScript`)